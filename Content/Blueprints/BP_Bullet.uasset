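; BP_Bullet is a projectile actor that destroys enemies on contact.
; Every tick, its Translate function moves it along its forward vector by Speed scaled by delta seconds, without sweeping.
; When it begins overlapping a BP_Enemy, it spawns an explosion emitter at its location, then destroys both the enemy and itself.
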(event EventBeginPlay)

(event Collision|EventActorBeginOverlap
  (params (OtherActor :type Actor%20Object%20Reference))
  ;[1 1 1] 충돌한 상대방이 플레이어라면 너죽고 나죽고 하고싶다.
  (Utilities|Casting|CastToBP_Enemy OtherActor)
  (Effects|SpawnEmitteratLocation "/Game/StarterContent/Particles/P_Explosion.P_Explosion" (Transformation|GetActorLocation))
  (Actor|DestroyActor OtherActor)
  (Actor|DestroyActor))

(event EventTick
  (params (DeltaSeconds :type Float%20%28single-precision%29))
  ;[1 1 1] 살아가면서 앞방향으로 계속 이동하고싶다.
  (CallFunction|Translate (Transformation|GetActorForwardVector) (Variables|Default|GetSpeed)))

(fn ConstructionScript)

(fn Translate
  (params (Direction :type Vector) (Speed :type Float%20%28double-precision%29))
  ;[1 1 1] P = P0 + velocity(dir * speed)*deltaSecond
  (Transformation|SetActorLocation (+ (Transformation|GetActorLocation) (* Direction Speed (Utilities|Time|GetWorldDeltaSeconds))) false false))