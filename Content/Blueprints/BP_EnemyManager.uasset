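; BP_EnemyManager is a spawner actor that creates BP_Enemy instances at a regular interval.
; BeginPlay starts a looping timer on SpawnTime that fires the SpawnEnemy event.
; SpawnEnemy places each enemy at the Spawn component's world location and rotation, always spawning regardless of collision.
; Two alternative periodic approaches, a delta-time accumulator and a Delay, remain in the graph but never run.
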(event Custom|SpawnEnemy
  (bind _spawn (Variables|Default|GetSpawn))
  (bind _returnvalue (Transformation|GetWorldTransform _spawn))
  (Game|SpawnActorfromClass "/Game/Blueprints/BP_Enemy.BP_Enemy_C" (Math|Transform|MakeTransform (.location _returnvalue) (.rotation _returnvalue) "1.000000,1.000000,1.000000") "AlwaysSpawn" "MultiplyWithRoot" 0 0))

(event EventBeginPlay
  ;[1 1 1] Timer를 이용한 주기
  (Utilities|Time|SetTimerbyEvent (delegate Custom|SpawnEnemy) (Variables|Default|GetSpawnTime) true))

(event Collision|EventActorBeginOverlap
  (params (OtherActor :type Actor%20Object%20Reference)))

(event EventTick
  (params (DeltaSeconds :type Float%20%28single-precision%29))
  ;[1 1 1] Delay를 이용한 주기
)

(fn ConstructionScript)