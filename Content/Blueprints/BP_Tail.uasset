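; BP_Tail is an actor that continuously follows a target actor, defaulting to the player.
; On BeginPlay, an invalid Target is replaced with the BP_Player found in the level.
; Each Tick moves it along the normalized direction to Target, scaled by Speed and delta time, without sweep.
; Target is not rechecked during Tick, and there is no stopping distance.
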(event EventBeginPlay
  ;[1 1 1] 태어날 때 목적지가 유효하지 않다면 주인공 플레이어를 목적지로 하고싶다.
  (Utilities|IsValid (Variables|Default|GetTarget)
    (:Is%20Not%20Valid
      (bind _returnvalue (Actor|GetActorOfClass "/Game/Blueprints/BP_Player.BP_Player_C"))
      (Variables|Default|SetTarget _returnvalue))))

(event Collision|EventActorBeginOverlap
  (params (OtherActor :type Actor%20Object%20Reference)))

(event EventTick
  (params (DeltaSeconds :type Float%20%28single-precision%29))
  ;[1 1 1] 살아가면서 목적지를 향해서 계속 이동하고싶다.
  (Transformation|SetActorLocation (+ (Transformation|GetActorLocation) (* (Math|Vector|Normalize (- (Transformation|GetActorLocation (Variables|Default|GetTarget)) (Transformation|GetActorLocation))) (Variables|Default|GetSpeed) (Utilities|Time|GetWorldDeltaSeconds))) false false))

(fn ConstructionScript)