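; BP_Player is a player actor that flies freely in a plane and shoots bullets.
; Each Tick it combines horizontal and vertical values along its right and up vectors, normalizes the result, and moves by direction, speed and delta time through a custom Translate function, without sweeping.
; The Fire input spawns BP_Bullet at the Arrow component's location and rotation, ignoring collisions.
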(event EventBeginPlay)

(event Collision|EventActorBeginOverlap
  (params (OtherActor :type Actor%20Object%20Reference)))

(event EventTick
  (params (DeltaSeconds :type Float%20%28single-precision%29))
  (CallFunction|Translate (Math|Vector|Normalize (+ (* (Transformation|GetActorRightVector) (Input|AxisValues|GetHorizontal)) (* (Transformation|GetActorUpVector) (Input|AxisValues|GetVertical)))) (Variables|Default|GetSpeed)))

(event Input|ActionEvents|InputActionFire
  (params (Key :type Key%20Structure :default "None"))
  (bind _arrow (Variables|Default|GetArrow))
  (bind _returnvalue (Transformation|GetWorldTransform _arrow))
  (:Pressed
    (Game|SpawnActorfromClass "/Game/Blueprints/BP_Bullet.BP_Bullet_C" (Math|Transform|MakeTransform (.location _returnvalue) (.rotation _returnvalue) "1.000000,1.000000,1.000000") "AlwaysSpawn" "MultiplyWithRoot" 0 0)))

(fn ConstructionScript)

(fn Translate
  (params (Direction :type Vector) (Speed :type Float%20%28double-precision%29))
  ;[1 1 1] P = P0 + velocity(dir * speed)*deltaSecond
  (Transformation|SetActorLocation (+ (Transformation|GetActorLocation) (* Direction Speed (Utilities|Time|GetWorldDeltaSeconds))) false false))