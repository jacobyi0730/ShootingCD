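; BP_Enemy is an enemy actor that flies in a straight line and destroys itself along with the player on contact.
; At BeginPlay it picks its direction once: 30% of the time toward the player's current position, otherwise its forward vector.
; Tick moves it along that stored direction, scaled by Speed and delta time, without sweeping.
; Overlapping BP_Player spawns an explosion emitter and destroys both actors.
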(event EventBeginPlay
  ;[1 1 1] 태어날때 이동할 방향을 기억하고싶다. 30%확률로 플레이어방향, 나머지확률로 앞방향으로 하고싶다.
  (if (< (Math|Random|RandomIntegerinRange 0 9) 3)
    (Variables|Default|SetDirection (Math|Vector|Normalize (- (Transformation|GetActorLocation (Game|Player|GetPlayerPawn 0)) (Transformation|GetActorLocation))))
    (else
      (Variables|Default|SetDirection (Transformation|GetActorForwardVector)))))

(event Collision|EventActorBeginOverlap
  (params (OtherActor :type Actor%20Object%20Reference))
  ;[1 1 1] 충돌한 상대방이 플레이어라면 너죽고 나죽고 하고싶다.
  (Utilities|Casting|CastToBP_Player OtherActor)
  (Effects|SpawnEmitteratLocation "/Game/StarterContent/Particles/P_Explosion.P_Explosion" (Transformation|GetActorLocation))
  (Actor|DestroyActor OtherActor)
  (Actor|DestroyActor))

(event EventTick
  (params (DeltaSeconds :type Float%20%28single-precision%29))
  ;[1 1 1] 기억하고 있는 방향으로 계속 이동하고싶다.
  (Transformation|SetActorLocation (+ (Transformation|GetActorLocation) (* (Variables|Default|GetDirection) (Variables|Default|GetSpeed) (Utilities|Time|GetWorldDeltaSeconds))) false false))

(fn ConstructionScript)